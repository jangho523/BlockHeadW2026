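; BP_Player is the player-controlled physics cube that runs forward through a level, dodging obstacles to reach the finish line.
; While the level is in play, Tick applies constant forward acceleration and Enhanced Input adds sideways force.
; Hitting an obstacle (after a delay) or falling below KillZ triggers death, while overlapping the finish line completes the level.
; Both outcomes notify BP_GameMode, with LevelInPlay gating them to fire once.
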(event OnComponentHit(Cube)
  (params (HitComponent :type Primitive%20Component%20Object%20Reference) (OtherActor :type Actor%20Object%20Reference) (OtherComp :type Primitive%20Component%20Object%20Reference) (NormalImpulse :type Vector :default "0, 0, 0") (Hit :type Hit%20Result%20Structure%20%28by%20ref%29))
  ;[0.15 0.8714 0.15 0.851] Hit Obstacle
  (Utilities|Casting|CastToBP_Obstacle OtherActor)
  (Utilities|FlowControl|Delay (Variables|LevelPlay|GetPostHitDelay))
  (CallFunction|PlayerDied))

(event OnComponentBeginOverlap(Cube)
  (params (OverlappedComponent :type Primitive%20Component%20Object%20Reference) (OtherActor :type Actor%20Object%20Reference) (OtherComp :type Primitive%20Component%20Object%20Reference) (OtherBodyIndex :type Integer) (bFromSweep :type Boolean) (SweepResult :type Hit%20Result%20Structure%20%28by%20ref%29))
  ;[0.15 0.8696 0.15 0.8522] Overlapped the Finish Line - Alert the Game Mode that the Level is Complete
  (Utilities|Casting|CastToBP_FinishLine OtherActor)
  (if (Variables|LevelPlay|GetbLevelInPlay)
    (Variables|LevelPlay|SetbLevelInPlay false)
    (Default|LevelComplete (Variables|Default|GetGameMode))))

(event Input|EnhancedActionEvents|EnhancedInputActionIA_MoveRightLeft
  (params (ActionValue :type Float%20%28double-precision%29) (ElapsedSeconds :type Float%20%28double-precision%29) (TriggeredSeconds :type Float%20%28double-precision%29) (InputAction :type Input%20Action%20Object%20Reference :default "/Game/BlockHead/Core/Input/Actions/IA_MoveRightLeft.IA_MoveRightLeft"))
  ;[0.15 0.8714 0.15 0.851] Movement
  (if (Variables|LevelPlay|GetbLevelInPlay)
    (Physics|AddForce (Variables|Default|GetCube) (* (Transformation|GetActorRightVector) (* ActionValue (Variables|Movement|GetSideForce))) "None" true)))

(event EventBeginPlay
  ;[0.15 0.8696 0.15 0.8522] Begin Play Sequence
  (Utilities|FlowControl|Sequence
    (:then_0
      ;[0.15 0.8714 0.15 0.851] Begin Play: Cast to the Player Controller and Add Mapping Context to the Input System
      (bind _asplayer_controller (Utilities|Casting|CastToPlayerController (Pawn|GetController)))
      (Variables|Default|SetPlayerController _asplayer_controller)
      (Input|AddMappingContext (PlayerController|LocalPlayerSubsystems|GetEnhancedInputLocalPlayerSubsystem (Variables|Default|GetPlayerController)) "/Game/BlockHead/Core/Input/IMC_Mappings.IMC_Mappings" 0 "(bIgnoreAllPressedKeysUntilRelease=True,bForceImmediately=False,bNotifyUserSettings=False)"))
    (:then_1
      ;[0.15 0.8696 0.15 0.8522] Get Reference to Game Mode
      (bind _asbp_game_mode (Utilities|Casting|CastToBP_GameMode (Game|GetGameMode)))
      (Variables|Default|SetGameMode _asbp_game_mode))))

(event EventTick
  (params (DeltaSeconds :type Float%20%28single-precision%29))
  ;[0.15 0.8696 0.15 0.8522] Event Tick Sequence
  (Utilities|FlowControl|Sequence
    (:then_0
      ;[0.15 0.8696 0.15 0.8522] Apply Forward Motion White Level is in Play
      (if (Variables|LevelPlay|GetbLevelInPlay)
        (Physics|AddForce (Variables|Default|GetCube) (* (Transformation|GetActorForwardVector) (Variables|Movement|GetForwardForce)) "None" true)))
    (:then_1
      (if (< (.z (Transformation|GetActorLocation)) (Variables|Default|GetKillZ))
        (CallFunction|PlayerDied)))))

(fn ConstructionScript)

(fn PlayerDied
  ;[0.15 0.8696 0.15 0.8522] Do Once
  (if (Variables|LevelPlay|GetbLevelInPlay)
    (Variables|LevelPlay|SetbLevelInPlay false)
    (Default|GameComplete (Variables|Default|GetGameMode) false)
    (return)))
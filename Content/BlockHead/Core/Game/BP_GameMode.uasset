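; BlockHead game mode that runs the level flow: score, level completion, win/lose end screen and restart.
; BeginPlay adds the HUD, caches the player and game instance, and sets game input.
; LevelComplete shows a widget, then a timer calls LoadNextLevel, which opens the next level or triggers the win screen on the final one.
; Level progression and input modes are delegated to BP_GameInstance, while score derives from the player's X position.
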(event EventBeginPlay
  ;[0.15 0.8696 0.15 0.8522] Begin Play Sequence
  (Utilities|FlowControl|Sequence
    (:then_0
      ;[0.15 0.8696 0.15 0.8522] Add HUD to Viewport
      (bind _returnvalue (UserInterface|CreateWidget "/Game/BlockHead/Core/UI/WBP_HUD.WBP_HUD_C"))
      (Variables|Default|SetHUD _returnvalue)
      (UserInterface|Viewport|AddtoViewport (Variables|Default|GetHUD) 0))
    (:then_1
      ;[0.15 0.8696 0.15 0.8522] Get Reference to Player Pawn
      (bind _asbp_player (Utilities|Casting|CastToBP_Player (Game|Player|GetPlayerPawn 0)))
      (Variables|Default|SetPlayer _asbp_player))
    (:then_2
      ;[0.15 0.8714 0.15 0.851] Get Reference to Game Instance
      (bind _asbp_game_instance (Utilities|Casting|CastToBP_GameInstance (Game|GetGameInstance)))
      (Variables|Default|SetGameInstance _asbp_game_instance))
    (:then_3
      ;[0.15 0.8714 0.15 0.851] Input Mode = Game
      (Default|InputModeGame (Variables|Default|GetGameInstance)))))

(fn ConstructionScript)

(fn GetScoreasText
  (return (|GenerictoText (Class|KismetMathLibrary|Round64 (/ (.x (Transformation|GetActorLocation (Variables|Default|GetPlayer))) 5e+02)))))

(fn LevelComplete
  ;[0.15 0.8714 0.15 0.851] Show Level Complete Widget and Set Timer for Loading Next Level
  (bind _returnvalue (UserInterface|CreateWidget "/Game/BlockHead/Core/UI/WBP_LevelComplete.WBP_LevelComplete_C"))
  (UserInterface|Viewport|AddtoViewport _returnvalue 0)
  (Utilities|Time|SetTimerbyFunctionName 0 "LoadNextLevel" 2.0)
  (return))

(fn LoadNextLevel
  (bind _bfinallevel (Default|IsPlayeronFinalLevel (Variables|Default|GetGameInstance)))
  (if _bfinallevel
    (CallFunction|GameComplete true)
    (else
      (Default|NextLevel (Variables|Default|GetGameInstance))
      (bind _levelname (Default|GetLevelName (Variables|Default|GetGameInstance)))
      (Game|OpenLevel(byName) _levelname)))
  (return))

(fn RestartGame
  ;[0.15 0.8714 0.15 0.851] Restart: Input Mode Set to Game. Reset Level Number and Load the First Level
  (Default|InputModeGame (Variables|Default|GetGameInstance))
  (Default|ResetInstance (Variables|Default|GetGameInstance))
  (bind _levelname (Default|GetLevelName (Variables|Default|GetGameInstance)))
  (Game|OpenLevel(byName) _levelname))

(fn GameComplete
  (params (bPlayerWon :type Boolean))
  ;[0.15 0.8714 0.15 0.851] Game is Complete - Show End Menu: Did Player Win or Lose?
  (if bPlayerWon
    (bind _returnvalue (UserInterface|CreateWidget "/Game/BlockHead/Core/UI/WBP_GameComplete.WBP_GameComplete_C" 0 "You Won! :)"))
    (UserInterface|Viewport|AddtoViewport _returnvalue 0)
    (else
      (bind _returnvalue_2 (UserInterface|CreateWidget "/Game/BlockHead/Core/UI/WBP_GameComplete.WBP_GameComplete_C" 0 "You Lost! :("))
      (UserInterface|Viewport|AddtoViewport _returnvalue_2 0)))
  (Default|InputModeUI (Variables|Default|GetGameInstance))
  (return))